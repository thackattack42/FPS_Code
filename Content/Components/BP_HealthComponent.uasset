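; Health component that tracks its owner's health and broadcasts hit, death and health-changed events.
; It starts at max health and listens to the owner's OnTakeAnyDamage.
; Damage types implementing BPI_DamageType can adjust damage using the component's ElementType before it is subtracted and clamped.
; At zero health it unbinds from damage and signals death; each processed hit also reports the health fraction.
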(event `self.ReceiveBeginPlay`
  ;[1 1 1] Comment
  (set `self.CurrentHealth` (`self.MaxHealth`))
  (add `Actor.OnTakeAnyDamage` (`self.GetOwner`) (`|CreateDelegate` :!event `DoDamage`)))

(event `DoDamage`
  (params (DamagedActor :type "Actor Object Reference") (Damage :type "Float (double-precision)") (DamageType :type "DamageType Object Reference") (InstigatedBy :type "Controller Object Reference") (DamageCauser :type "Actor Object Reference"))
  (bind _newdamage (`self.GetDamage` DamageType Damage))
  ;[1 1 1] Comment
  (bind _output_get (set `self.CurrentHealth` (`KismetMathLibrary.FClamp` (- (`self.CurrentHealth`) _newdamage) 0.0 (`self.MaxHealth`))))
  (if (> _output_get 0.0)
    (`self.OnHit`)
    (else
      (remove `Actor.OnTakeAnyDamage` (`self.GetOwner`) (`|CreateDelegate` :!event `DoDamage`))
      (`self.OnDeath`)))
  (`self.OnHealthChanged` (/ (`self.CurrentHealth`) (`self.MaxHealth`))))

(fn `GetDamage`
  (params (TestObject :type "Object Object Reference") (Damage :type "Float (double-precision)"))
  (returns (NewDamage :type "Float (double-precision)"))
  (if (`KismetSystemLibrary.DoesImplementInterface` TestObject "/Game/Utility/BPI_DamageType.BPI_DamageType_C")
    (bind _newdamage (message `/Game/Utility/BPI_DamageType.HandleDamageType` TestObject (`self.ElementType`) Damage))
    (return _newdamage)
    (else
      (return Damage))))