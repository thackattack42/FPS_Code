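; Base rifle weapon actor that expects a Pawn as its parent actor and fires projectiles on that pawn's behalf.
; Attack checks CanShoot (not busy, not dead, has ammo), then spawns the bullet class at a mesh socket along the pawn's aim rotation.
; Each shot sets the busy flag, starts a timer, broadcasts the shot and spends ammo; StopProcess is empty.
; Ammo use and Reload broadcast ammo changes, and OwnerDead disables firing.
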(event `self.ReceiveBeginPlay`
  ;[1 1 1] Done
  (bind _aspawn (cast `Pawn` (`self.GetParentActor`))
    (:`then`
      (set `self.ParentPawn` _aspawn))
    (:`CastFailed`
      (`KismetSystemLibrary.PrintString` "We need a pawn to spawn this weapon"))))

(event `OwnerDead`
  (set `self.Dead` true))

(event `Reload`
  ;[1 1 1] Comment
  (bind _output_get (set `self.CurrentAmmo` (`self.MaxAmmo`)))
  (`self.OnAmmoChanged` _output_get (`self.MaxAmmo`)))

(event `UseAmmo`
  (params (DeltaTime :type "Float (double-precision)"))
  (bind _result (`/Engine/EditorBlueprintResources/StandardMacros.DecrementFloat` (`self.CurrentAmmo`))
    (:`  `
      (bind _output_get (set `self.CurrentAmmo` (`KismetMathLibrary.FMax` _result)))
      (`self.OnAmmoChanged` _output_get (`self.MaxAmmo`)))))

(fn `Attack`
  (bind _parentpawn (`self.ParentPawn`))
  (if (`self.CanShoot`)
    (`|SpawnActorFromClass` (`self.BulletClass`) (`KismetMathLibrary.MakeTransform` (`SceneComponent.GetSocketLocation` (`self.SkeletalMesh`) (`self.SocketName`)) (`Pawn.GetBaseAimRotation` _parentpawn)) "Undefined" "OverrideRootScale" null _parentpawn)
    (set `self.InProcess` true)
    (`self.OnShotHappened`)
    (`KismetSystemLibrary.K2_SetTimerDelegate` (`|CreateDelegate` :!event `StopProcess`) 2.0)
    (`self.UseAmmo` 0.0)))

(fn `CanShoot`
  (returns (ReturnValue :type Boolean))
  ;[1 1 1] Done
  (return (and (not (`self.InProcess`)) (not (`self.Dead`)) (> (`self.CurrentAmmo`) 0.0))))

(fn `StopProcess`)

(fn `UserConstructionScript`)