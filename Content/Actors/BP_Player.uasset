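; Player character Blueprint that handles first-hand input for movement, looking, attacking and reloading its current weapon.
; On BeginPlay it creates the on-screen widget and binds health component events, destroying itself without a player controller.
; Movement follows control yaw, while reload also triggers the animation Blueprint.
; HandleDeath disables input, then binds the weapon's ammo-change event and calls Reload.
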(event `self.ReceiveBeginPlay`
  (`parent.ReceiveBeginPlay`)
  (bind _asplayer_controller (cast `PlayerController` (`self.GetController`))
    (:`then`
      (bind _output_get (set `self.PlayerController` _asplayer_controller))
      (bind _returnvalue (`|CreateWidget` (`self.WidgetClass`) _output_get))
      (`UserWidget.AddToViewport` _returnvalue 0)
      (add `/Game/Components/BP_HealthComponent.OnHealthChanged` (`self.BP_HealthComponent`) (`|CreateDelegate` _returnvalue :!event `SetHealth`))
      (add `/Game/Components/BP_HealthComponent.OnDeath` (`self.BP_HealthComponent`) (delegate `HandleDeath`)))
    (:`CastFailed`
      (`KismetSystemLibrary.PrintString` "Needs a player comtroller")
      (`self.K2_DestroyActor`))))

(event `HandleDeath`
  (bind _currentweapon (`self.CurrentWeapon`))
  (`parent.HandleDeath`)
  (`self.DisableInput` (`self.PlayerController`))
  (add `/Game/Actors/BP_BaseRifle.OnAmmoChanged` _currentweapon (`|CreateDelegate` (stale `self.ReceiveBeginPlay` _returnvalue) :!event `SetAmmo`))
  (`/Game/Actors/BP_BaseRifle.Reload` _currentweapon))

(event `InputAxis|TurnTo`
  (params (AxisValue :type "Float (single-precision)"))
  ;[1 1 1] Comment
  (`self.AddControllerYawInput` AxisValue))

(event `InputAxis|LookUp`
  (params (AxisValue :type "Float (single-precision)"))
  ;[1 1 1] Comment
  (`self.AddControllerPitchInput` AxisValue))

(event `InputAction|Reload`
  (params (Key :type "Key Structure"))
  (:`Pressed`
    (`/Game/Actors/BP_BaseRifle.Reload` (`self.CurrentWeapon`))
    (`/Game/CodeBase/ABP_BaseCharacter.ReloadAnimation` (`self.AnimBP`))))

(event `InputAxis|Forward`
  (params (AxisValue :type "Float (single-precision)"))
  (bind (_returnvalue_roll _returnvalue_pitch _returnvalue_yaw) (`KismetMathLibrary.BreakRotator` (`self.GetControlRotation`)))
  ;[1 1 1] Comment
  (`self.AddMovementInput` (`KismetMathLibrary.GetForwardVector` (`KismetMathLibrary.MakeRotator` 0.0 0.0 _returnvalue_yaw)) AxisValue))

(event `InputAxis|Right`
  (params (AxisValue :type "Float (single-precision)"))
  (bind (_returnvalue_roll _returnvalue_pitch _returnvalue_yaw) (`KismetMathLibrary.BreakRotator` (`self.GetControlRotation`)))
  ;[1 1 1] Comment
  (`self.AddMovementInput` (`KismetMathLibrary.GetRightVector` (`KismetMathLibrary.MakeRotator` 0.0 0.0 _returnvalue_yaw)) AxisValue))

(event `InputAction|Attack`
  (params (Key :type "Key Structure"))
  (:`Pressed`
    (`self.CharacterAttack`)))

(fn `UserConstructionScript`
  (`parent.UserConstructionScript`))