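; Base character Blueprint that carries a weapon, can attack with it, and handles hits and death.
; On BeginPlay it spawns the weapon class via a child actor, caches the rifle and anim blueprint, and binds shot, shoot-end, hit and death events, destroying itself if either cast fails.
; CharacterAttack forwards to the weapon.
; Death plays the dead animation, notifies the weapon and disables collision.
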(event `self.ReceiveBeginPlay`
  (bind _weaponchildactorcomponent (`self.WeaponChildActorComponent`))
  (bind _bp_healthcomponent (`self.BP_HealthComponent`))
  ;[1 1 1] Comment
  (`ChildActorComponent.SetChildActorClass` _weaponchildactorcomponent (`self.Weapon Class`))
  (bind _asbp_base_rifle (cast `/Game/Actors/BP_BaseRifle` (`ChildActorComponent.ChildActor` _weaponchildactorcomponent))
    (:`then`
      (set `self.CurrentWeapon` _asbp_base_rifle)
      (bind _asabp_base_character (cast `/Game/CodeBase/ABP_BaseCharacter` (`SkeletalMeshComponent.GetAnimInstance` (`self.Mesh`)))
        (:`then`
          (set `self.AnimBP` _asabp_base_character)
          (add `/Game/Actors/BP_BaseRifle.OnShotHappened` (`self.CurrentWeapon`) (`|CreateDelegate` (`self.AnimBP`) :!event `FireAnimation`))
          (add `/Game/CodeBase/ABP_BaseCharacter.OnShootEnd` (`self.AnimBP`) (`|CreateDelegate` (`self.CurrentWeapon`) :!event `StopProcess`))
          (add `/Game/Components/BP_HealthComponent.OnHit` _bp_healthcomponent (`|CreateDelegate` (`self.AnimBP`) :!event `HitAnimation`))
          (add `/Game/Components/BP_HealthComponent.OnDeath` _bp_healthcomponent (`|CreateDelegate` :!event `HandleDeath`)))
        (:`CastFailed`
          (`KismetSystemLibrary.PrintString` "We have to set out anim to correct type")
          (`self.K2_DestroyActor`))))
    (:`CastFailed`
      (`KismetSystemLibrary.PrintString` "There is no weapon will crash")
      (`self.K2_DestroyActor`))))

(event `HandleDeath`
  (`/Game/CodeBase/ABP_BaseCharacter.DeadAnimation` (`self.AnimBP`))
  (`/Game/Actors/BP_BaseRifle.OwnerDead` (`self.CurrentWeapon`))
  (`self.SetActorEnableCollision` false))

(fn `CharacterAttack`
  (`/Game/Actors/BP_BaseRifle.Attack` (`self.CurrentWeapon`)))

(fn `UserConstructionScript`)